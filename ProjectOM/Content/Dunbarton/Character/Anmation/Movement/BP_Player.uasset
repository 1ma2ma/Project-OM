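; BP_Player is the player Blueprint that handles basic movement and camera look from axis inputs.
; Forward and right inputs move it along the capsule's forward and right vectors, scaled by a movement multiplier and frame delta seconds.
; LookUp and Turn inputs add controller pitch and yaw, scaled by a sensitivity value without delta time.
; The construction script is empty.
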(event `InputAxis|MoveForward`
  (params (AxisValue :type "Float (single-precision)"))
  (`self.AddMovementInput` (`SceneComponent.GetForwardVector` (`self.CapsuleComponent`)) (* AxisValue (`self.MovementMultplayer`) (`GameplayStatics.GetWorldDeltaSeconds`))))

(event `InputAxis|MoveRight`
  (params (AxisValue :type "Float (single-precision)"))
  (`self.AddMovementInput` (`SceneComponent.GetRightVector` (`self.CapsuleComponent`)) (* AxisValue (`self.MovementMultplayer`) (`GameplayStatics.GetWorldDeltaSeconds`))))

(event `InputAxis|LookUp`
  (params (AxisValue :type "Float (single-precision)"))
  (`self.AddControllerPitchInput` (* AxisValue (`self.MoveSensitivity`))))

(event `InputAxis|Turn`
  (params (AxisValue :type "Float (single-precision)"))
  (`self.AddControllerYawInput` (* AxisValue (`self.MoveSensitivity`))))

(fn `UserConstructionScript`)